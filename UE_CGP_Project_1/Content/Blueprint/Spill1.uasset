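; Spill1 is a cleanable spill actor that the player removes by holding the left mouse button while inside its box collider.
; Overlap with SpongeCharacter enables input on the spill, and leaving disables it.
; Holding the button plays a timeline driving Opacity2 in the Spill_Collection material parameter collection; releasing pauses it.
; The actor destroys itself when the timeline finishes.
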(event OnComponentBeginOverlap(Box)
  (params (OverlappedComponent :type Primitive%20Component%20Object%20Reference) (OtherActor :type Actor%20Object%20Reference) (OtherComp :type Primitive%20Component%20Object%20Reference) (OtherBodyIndex :type Integer) (bFromSweep :type Boolean) (SweepResult :type Hit%20Result%20Structure%20%28by%20ref%29))
  ;[1 1 1] Allow to be clean only if player is touching the collider
  (Utilities|Casting|CastToSpongeCharacter OtherActor)
  (Development|PrintString "collide")
  (Input|EnableInput (Game|GetPlayerController 0)))

(event OnComponentEndOverlap(Box)
  (params (OverlappedComponent :type Primitive%20Component%20Object%20Reference) (OtherActor :type Actor%20Object%20Reference) (OtherComp :type Primitive%20Component%20Object%20Reference) (OtherBodyIndex :type Integer))
  ;[1 1 1] Allow to be clean only if player is touching the collider
  (Utilities|Casting|CastToSpongeCharacter OtherActor)
  (Development|PrintString "no longer collide")
  (Input|DisableInput (Game|GetPlayerController 0)))

(event Input|MouseEvents|LeftMouseButton
  (params (Key :type Key%20Structure :default "None"))
  ;[1 1 1] Making the spill transparent and destroy once timeline finished
  (:Pressed
    (bind _opacity (Timeline|Timeline_0 Play)
      (:Update
        (Rendering|Material|SetScalarParameterValue "/Game/Blueprint/Collection/Spill_Collection.Spill_Collection" "Opacity2" _opacity :!class /Script/Engine.KismetMaterialLibrary))
      (:Finished
        (Actor|DestroyActor))))
  (:Released
    (Timeline|Timeline_0 Stop)))

(fn ConstructionScript)