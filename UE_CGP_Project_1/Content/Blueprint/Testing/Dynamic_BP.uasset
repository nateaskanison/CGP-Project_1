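; Test actor that lets the player fade its mesh colour with a key while a HandCharacter overlaps its collider.
; On overlap it creates a dynamic instance of Test_M on the static mesh and enables input, which it disables when the overlap ends.
; Holding the 1 key plays the ChangeColor timeline, driving the material's Colour parameter; releasing stops it.
; Print strings trace each step.
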(event OnComponentBeginOverlap(Collider)
  (params (OverlappedComponent :type Primitive%20Component%20Object%20Reference) (OtherActor :type Actor%20Object%20Reference) (OtherComp :type Primitive%20Component%20Object%20Reference) (OtherBodyIndex :type Integer) (bFromSweep :type Boolean) (SweepResult :type Hit%20Result%20Structure%20%28by%20ref%29))
  (Utilities|Casting|CastToHandCharacter OtherActor)
  (Development|PrintString "colliding")
  (bind _returnvalue (Rendering|Material|CreateDynamicMaterialInstance (Variables|Default|GetStaticMesh) 0 "/Game/Blueprint/Testing/Test_M.Test_M" "None" :!class /Script/Engine.PrimitiveComponent))
  (Input|EnableInput (Game|GetPlayerController 0)))

(event OnComponentEndOverlap(Collider)
  (params (OverlappedComponent :type Primitive%20Component%20Object%20Reference) (OtherActor :type Actor%20Object%20Reference) (OtherComp :type Primitive%20Component%20Object%20Reference) (OtherBodyIndex :type Integer))
  (Utilities|Casting|CastToHandCharacter OtherActor)
  (Development|PrintString "no longer collide")
  (Input|DisableInput (Game|GetPlayerController 0)))

(event Input|KeyboardEvents|1
  (params (Key :type Key%20Structure :default "None"))
  (:Pressed
    (Development|PrintString "changing color")
    (bind _colour_fade (Timeline|Change%20color Play)
      (:Update
        (Rendering|Material|SetVectorParameterValue (stale OnComponentBeginOverlap(Collider) _returnvalue) "Colour" _colour_fade :!class /Script/Engine.MaterialInstanceDynamic))))
  (:Released
    (Development|PrintString "stoped")
    (Timeline|Change%20color Stop)))

(fn ConstructionScript)