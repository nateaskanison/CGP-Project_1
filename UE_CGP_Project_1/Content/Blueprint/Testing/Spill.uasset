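; Test Blueprint for a spill that reacts to a HandCharacter, apparently an unfinished prototype of cleaning it up.
; Box overlap enables player input on the actor and calls dynamic material creation with an unused result; leaving disables input, with debug prints for both.
; Cleaning prints and the swap to Fade_Material on the Spill component are unwired, with a note to change to mouse press.
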(event OnComponentBeginOverlap(Box)
  (params (OverlappedComponent :type Primitive%20Component%20Object%20Reference) (OtherActor :type Actor%20Object%20Reference) (OtherComp :type Primitive%20Component%20Object%20Reference) (OtherBodyIndex :type Integer) (bFromSweep :type Boolean) (SweepResult :type Hit%20Result%20Structure%20%28by%20ref%29))
  (Utilities|Casting|CastToHandCharacter OtherActor)
  (Development|PrintString "colliding")
  (Rendering|Material|CreateDynamicMaterialInstance 0 "None" "None" :!class /Script/Engine.KismetMaterialLibrary)
  (Input|EnableInput (Game|GetPlayerController 0)))

(event OnComponentEndOverlap(Box)
  (params (OverlappedComponent :type Primitive%20Component%20Object%20Reference) (OtherActor :type Actor%20Object%20Reference) (OtherComp :type Primitive%20Component%20Object%20Reference) (OtherBodyIndex :type Integer))
  (Utilities|Casting|CastToHandCharacter OtherActor)
  (Development|PrintString "not colliding")
  (Input|DisableInput (Game|GetPlayerController 0)))

(event Input|KeyboardEvents|1
  (params (Key :type Key%20Structure :default "None")))

(fn ConstructionScript)