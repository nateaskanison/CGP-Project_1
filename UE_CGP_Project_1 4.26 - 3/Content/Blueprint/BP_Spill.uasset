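; Cleanable spill actor that the sponge character scrubs away with the PlayerClean input.
; Box overlap with SpongeCharacter toggles the actor's input, so cleaning works only while touching it.
; Holding the input plays a timeline fading material opacity and activates the character's particles; releasing or leaving stops both.
; When the timeline finishes, CallUITrigger lowers the level manager's count and the spill is destroyed.
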(event OnComponentBeginOverlap(Box)
  (params (OverlappedComponent :type Primitive%20Component%20Object%20Reference) (OtherActor :type Actor%20Object%20Reference) (OtherComp :type Primitive%20Component%20Object%20Reference) (OtherBodyIndex :type Integer) (bFromSweep :type Boolean) (SweepResult :type Hit%20Result%20Structure%20%28by%20ref%29))
  ;[1 1 1] Allow to be clean only if player is touching the collider
  (Utilities|Casting|CastToSpongeCharacter OtherActor)
  (Development|PrintString "collide")
  (Input|EnableInput (Game|GetPlayerController 0)))

(event OnComponentEndOverlap(Box)
  (params (OverlappedComponent :type Primitive%20Component%20Object%20Reference) (OtherActor :type Actor%20Object%20Reference) (OtherComp :type Primitive%20Component%20Object%20Reference) (OtherBodyIndex :type Integer))
  ;[1 1 1] Allow to be clean only if player is touching the collider
  (bind _assponge_character (Utilities|Casting|CastToSpongeCharacter OtherActor))
  (Development|PrintString "no longer collide")
  (Input|DisableInput (Game|GetPlayerController 0))
  (Default|DeactiveParticle _assponge_character) ; stop particle from keep playing when player exit the spill
  ;[1 1 1] Making the spill transparent and destroy once timeline finished
  (bind _opacity (Timeline|Timeline_0 Stop)
    (:Update
      (Rendering|Material|SetScalarParameterValueonMaterials (Variables|Default|GetStaticMesh) "Opacity" (Math|Float|Lerp 0.0 1.0 _opacity)) ; Set material of mesh the opacity
    )
    (:Finished
      (Default|CallUITrigger) ; calling lower count from level manager
      (Actor|DestroyActor) ; destroy spill once finished timeline
    )))

(event Input|ActionEvents|InputActionPlayerClean
  (params (Key :type Key%20Structure :default "None"))
  ;[1 1 1] Making the spill transparent and destroy once timeline finished
  (:Pressed
    (bind _opacity (Timeline|Timeline_0 Play)
      (:Update
        (Rendering|Material|SetScalarParameterValueonMaterials (Variables|Default|GetStaticMesh) "Opacity" (Math|Float|Lerp 0.0 1.0 _opacity)) ; Set material of mesh the opacity
      )
      (:Finished
        (Default|CallUITrigger) ; calling lower count from level manager
        (Actor|DestroyActor) ; destroy spill once finished timeline
      )))
  (:Released
    (Timeline|Timeline_0 Stop)))

(event Input|ActionEvents|InputActionPlayerClean
  (params (Key :type Key%20Structure :default "None"))
  (bind _returnvalue (Game|GetPlayerCharacter 0))
  ;[1 1 1] Play Particle when player click to clean
  (:Pressed
    (bind _assponge_character (Utilities|Casting|CastToSpongeCharacter _returnvalue))
    (Default|ActivateParticle _assponge_character))
  (:Released
    (bind _assponge_character_2 (Utilities|Casting|CastToSpongeCharacter _returnvalue))
    (Default|DeactiveParticle _assponge_character_2)))

(fn ConstructionScript)